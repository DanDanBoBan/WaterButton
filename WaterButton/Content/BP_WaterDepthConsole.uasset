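; BP_WaterDepthConsole is a console that raises or lowers an actor, named as water, between preset depth levels.
; RaiseWater and LowerWater step a level index clamped to the ActorLocations array, then smoothly move ActorToMove's root to that reference actor's location and rotation with an eased MoveComponentTo.
; Begin and end overlap events show its text render only while a pawn overlaps the console.
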(event Custom|RaiseWater
  (Math|Integer|IncrementInt (Variables|Default|GetWaterDestinationLevel)
    (:%20%20
      (Variables|Default|SetWaterDestinationLevel (Math|Integer|Clamp(Integer) (Variables|Default|GetWaterDestinationLevel) 0 (Utilities|Array|LastIndex (Variables|Default|GetActorLocations))))
      (Components|MoveComponentTo (Variables|/Script/Engine.Actor|GetRootComponent (Variables|Default|GetActorToMove)) (Transformation|GetActorLocation (Utilities|Array|Get(acopy) (Variables|Default|GetActorLocations) (Variables|Default|GetWaterDestinationLevel))) (Transformation|GetActorRotation (Utilities|Array|Get(acopy) (Variables|Default|GetActorLocations) (Variables|Default|GetWaterDestinationLevel))) true true 1.0 false))))

(event Custom|LowerWater
  (Math|Integer|DecrementInt (Variables|Default|GetWaterDestinationLevel)
    (:%20%20
      (Variables|Default|SetWaterDestinationLevel (Math|Integer|Clamp(Integer) (Variables|Default|GetWaterDestinationLevel) 0 (Utilities|Array|LastIndex (Variables|Default|GetActorLocations))))
      (Components|MoveComponentTo (Variables|/Script/Engine.Actor|GetRootComponent (Variables|Default|GetActorToMove)) (Transformation|GetActorLocation (Utilities|Array|Get(acopy) (Variables|Default|GetActorLocations) (Variables|Default|GetWaterDestinationLevel))) (Transformation|GetActorRotation (Utilities|Array|Get(acopy) (Variables|Default|GetActorLocations) (Variables|Default|GetWaterDestinationLevel))) true true 1.0 false))))

(event EventBeginPlay)

(event Collision|EventActorBeginOverlap
  (params (OtherActor :type Actor%20Object%20Reference))
  (Development|SetHiddeninGame (Variables|Default|GetTextRender) (Utilities|Array|IsEmpty (Collision|GetOverlappingActors "/Script/Engine.Pawn" :!class /Script/Engine.Actor)) false))

(event EventTick
  (params (DeltaSeconds :type Float%20%28single-precision%29)))

(event Collision|EventActorEndOverlap
  (params (OtherActor :type Actor%20Object%20Reference))
  (Development|SetHiddeninGame (Variables|Default|GetTextRender) (Utilities|Array|IsEmpty (Collision|GetOverlappingActors "/Script/Engine.Pawn" :!class /Script/Engine.Actor)) false))

(fn ConstructionScript)